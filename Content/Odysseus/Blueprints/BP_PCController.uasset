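; BP_PCController is a controller Blueprint that opens the game's pause menu.
; When the Pause input is pressed, it creates a UMG_Pause widget only if no valid reference exists, so later presses reuse the same instance.
; It then shows the mouse cursor, switches to UI-only input focused on the widget, adds it to the viewport and pauses the game.
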(event Input|ActionEvents|InputActionPause
  (params (Key :type Key%20Structure :default "None"))
  (bind _returnvalue (Game|GetPlayerController 0))
  ;[1 1 1] Call Pause Widget
  (:Pressed
    (Utilities|IsValid (Variables|Default|GetPause%20Reference)
      (:Is%20Valid
        _)
      (:Is%20Not%20Valid
        (bind _returnvalue_2 (UserInterface|CreateWidget "/Game/Odysseus/Blueprints/BP_UI/UMG_Pause.UMG_Pause_C" (Game|GetPlayerController 0)))
        (Variables|Default|SetPause%20Reference _returnvalue_2)))
    (Variables|/Script/Engine.PlayerController|SetbShowMouseCursor _returnvalue true)
    (Input|SetInputModeUIOnly _returnvalue (Variables|Default|GetPause%20Reference) "DoNotLock")
    (UserInterface|Viewport|AddtoViewport (Variables|Default|GetPause%20Reference) 0)
    (Game|SetGamePaused true)))

(fn ConstructionScript)